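; BP_Lore is a lore trigger actor that shows a text widget while the player is inside it.
; On BeginPlay it creates a WBP_Lore widget and copies its Text variable into the widget's text block.
; Overlap by the player pawn adds the widget to the viewport, and leaving the Box component removes it.
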(event `self.ReceiveActorBeginOverlap`
  (params (OtherActor :type "Actor Object Reference"))
  (if (== OtherActor (`GameplayStatics.GetPlayerPawn` 0))
    (`UserWidget.AddToViewport` (`self.Widget`) 0)))

(event `self.ReceiveBeginPlay`
  (bind _returnvalue (`|CreateWidget` "/Game/Blueprint/WBP_Lore.WBP_Lore_C"))
  (bind _output_get (set `self.Widget` _returnvalue))
  (bind _aswbp_lore (cast `/Game/Blueprint/WBP_Lore` _output_get))
  (set `TextBlock.Text` (`self.Text`) (`/Game/Blueprint/WBP_Lore.Text` _aswbp_lore)))

(event `self.Box.OnComponentEndOverlap`
  (params (OverlappedComponent :type "PrimitiveComponent Object Reference") (OtherActor :type "Actor Object Reference") (OtherComp :type "PrimitiveComponent Object Reference") (OtherBodyIndex :type Integer))
  (if (== OtherActor (`GameplayStatics.GetPlayerPawn` 0))
    (`Widget.RemoveFromParent` (`self.Widget`))))

(fn `UserConstructionScript`)