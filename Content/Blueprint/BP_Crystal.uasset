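; BP_Crystal is a crystal actor that the player triggers by overlapping it.
; On overlap with player pawn 0, it passes itself to that pawn through AddCrystalMessage.
; Its UpdateMesh event disables actor collision and hides the point light and StaticMesh2, leaving the actor in the level rather than destroying it.
; Nothing in this Blueprint calls UpdateMesh.
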(event `self.ReceiveActorBeginOverlap`
  (params (OtherActor :type "Actor Object Reference"))
  (bind _returnvalue (`GameplayStatics.GetPlayerPawn` 0))
  (if (== OtherActor _returnvalue)
    (message `/Game/Blueprint/Interfaces/BPI_Crystal.AddCrystal` _returnvalue self)))

(event `/Game/Blueprint/Interfaces/BPI_Crystal.UpdateMesh`
  (`self.SetActorEnableCollision` false)
  (`SceneComponent.SetVisibility` (`self.PointLight`) false false)
  (`SceneComponent.SetVisibility` (`self.StaticMesh2`) false false))

(fn `UserConstructionScript`)