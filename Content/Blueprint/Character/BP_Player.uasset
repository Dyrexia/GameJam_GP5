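; BP_Player is the player character, which moves via Enhanced Input, collects crystals and keys, and can shine a battery-powered light.
; Movement input also sets facing yaw, and is blocked while the light shines.
; Shining spends one battery charge and plays a timeline animating point light radius, intensity and camera height.
; Crystals recharge the battery up to its maximum, key IDs are stored for door checks, and Kill only prints a debug message.
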(event `self.ReceivePossessed`
  (params (NewController :type "Controller Object Reference"))
  (bind _asplayer_controller (cast `PlayerController` NewController))
  (`EnhancedInputSubsystemInterface.AddMappingContext` (pcsubsystem `EnhancedInputLocalPlayerSubsystem` _asplayer_controller) "/Game/Blueprint/Inputs/IMC_Player.IMC_Player" 0 (struct)))

(event `EnhancedInput|/Game/Blueprint/Inputs/Actions/IA_Move`
  (params (ActionValue :type "Vector2D Structure") (ElapsedSeconds :type "Float (double-precision)") (TriggeredSeconds :type "Float (double-precision)") (InputAction :type "InputAction Object Reference" :default "/Game/Blueprint/Inputs/Actions/IA_Move.IA_Move"))
  (bind (_x _y) (`KismetMathLibrary.BreakVector2D` ActionValue))
  (bind (_x_2 _y_2) (`KismetMathLibrary.BreakVector2D` (`KismetMathLibrary.Normal2D` ActionValue)))
  (:`Triggered`
    (if (not (`self.IsShiningLight?`))
      (`self.AddMovementInput` (`KismetMathLibrary.Conv_Vector2DToVector` ActionValue))
      (if (and (== _x -1.0) (== _y 0.0))
        (`self.K2_SetActorRotation` (`KismetMathLibrary.MakeRotator` 0.0 0.0 180.0))
        (else
          (`self.K2_SetActorRotation` (`KismetMathLibrary.MakeRotator` 0.0 0.0 (* (`KismetMathLibrary.DegAcos` _x_2) (`KismetMathLibrary.SignOfFloat` _y_2)))))))))

(event `/Game/Blueprint/Interfaces/BPI_Kill.Kill`
  (`KismetSystemLibrary.PrintString` "Am ded" true true (struct :`G` 0.66 :`B` 1.0 :`A` 1.0) 2.0 "ded"))

(event `EnhancedInput|/Game/Blueprint/Inputs/Actions/IA_ShineLight`
  (params (ActionValue :type Boolean) (ElapsedSeconds :type "Float (double-precision)") (TriggeredSeconds :type "Float (double-precision)") (InputAction :type "InputAction Object Reference" :default "/Game/Blueprint/Inputs/Actions/IA_ShineLight.IA_ShineLight"))
  (bind _pointlight (`self.PointLight`))
  (:`Started`
    (if (> (`self.Battery`) 0)
      (`/Engine/EditorBlueprintResources/StandardMacros.DecrementInt` (`self.Battery`)
        (:`  `
          (set `self.IsShiningLight?` true)
          (bind (_direction _lightradius _cameraheight _lightstrength) (`Timeline|ShineLight` :!via `PlayFromStart`)
            (:`Update`
              (`LocalLightComponent.SetAttenuationRadius` _pointlight _lightradius)
              (`LightComponent.SetIntensity` _pointlight _lightstrength)
              (`SceneComponent.K2_SetRelativeLocation` (`self.Camera`) (`KismetMathLibrary.MakeVector` 0.0 0.0 _cameraheight) false false))
            (:`Finished`
              (set `self.IsShiningLight?` false))))))))

(event `/Game/Blueprint/Interfaces/BPI_Crystal.AddCrystal`
  (params (CrystalRef :type "Actor Object Reference"))
  (if (< (`self.Battery`) (`self.MaxBattery`))
    (bind _result (`/Engine/EditorBlueprintResources/StandardMacros.IncrementInt` (`self.Battery`))
      (:`  `
        (message `/Game/Blueprint/Interfaces/BPI_Crystal.UpdateMesh` CrystalRef)
        (`KismetSystemLibrary.PrintString` (`KismetStringLibrary.Conv_IntToString` _result))))))

(event `/Game/Blueprint/Interfaces/BPI_Key.AddKey`
  (params (KeyID :type Integer))
  (`KismetArrayLibrary.Array_Add` (`self.Keys`) KeyID))

(fn `GetIsShiningLight`
  (returns (IsShinningLight :type Boolean))
  (return (`self.IsShiningLight?`)))

(fn `TestPlayerKeys`
  (params (DoorID :type Integer))
  (returns (HasKeys :type Boolean))
  (return (`KismetArrayLibrary.Array_Contains` (`self.Keys`) DoorID)))

(fn `UserConstructionScript`)